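; BP_Gun is an automatic gun weapon that simulates physics until attached, when it disables physics and enables player input.
; Holding Fire calls Firing immediately and then on a looping timer until release.
; Firing traces from the camera to find the aim point, then spawns a BP_Bullet at the muzzle offset, rotated toward that point so shots converge on the crosshair.
; Detaching restores physics and disables input.
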(event Custom|BeforeDettached
  (Physics|SetSimulatePhysics (Variables|Default|GetStaticMesh) true)
  (Input|DisableInput (Pawn|GetLocalViewingPlayerController (Game|Player|GetPlayerPawn 0))))

(event Custom|BeforeAttached
  (Physics|SetSimulatePhysics (Variables|Default|GetStaticMesh) false)
  (Input|EnableInput (Pawn|GetLocalViewingPlayerController (Game|Player|GetPlayerPawn 0))))

(event EventBeginPlay
  (Physics|SetSimulatePhysics (Variables|Default|GetStaticMesh) true))

(event Input|ActionEvents|InputActionFire
  (params (Key :type Key%20Structure :default "None"))
  (:Pressed
    (CallFunction|Firing)
    (bind _returnvalue (Utilities|Time|SetTimerbyFunctionName 0 "Firing" 0.1 true)))
  (:Released
    (Utilities|Time|ClearandInvalidateTimerbyHandle _returnvalue)))

(fn ConstructionScript
  (|CallParentFunction))

(fn Firing
  (bind _returnvalue (Game|GetPlayerCameraManager 0))
  (bind _staticmesh (Variables|Default|GetStaticMesh))
  (bind _transformcomponent (Variables|/Script/Engine.PlayerCameraManager|GetTransformComponent _returnvalue))
  (bind _returnvalue_2 (Transformation|GetWorldLocation _transformcomponent))
  (bind _outhit (Collision|LineTraceByChannel _returnvalue_2 (+ _returnvalue_2 (* (Math|Vector|GetForwardVector _transformcomponent) 1e+05)) "TraceTypeQuery1" true 0 "None"))
  (bind _outhit_2 (Collision|LineTraceByChannel (+ (Transformation|GetWorldLocation _staticmesh) (Math|Vector|RotateVector (Variables|Default|GetGunMuzzleOffset) (Transformation|GetWorldRotation _staticmesh))) (select (.bblockinghit _outhit) (.impactpoint _outhit) (.traceend _outhit)) "TraceTypeQuery1" false 0 "None"))
  (Game|SpawnActorfromClass "/Game/WeaponSystem/Blueprint/Weapon/BP_Bullet.BP_Bullet_C" (Math|Transform|MakeTransform (.tracestart _outhit_2) (Math|Rotator|FindLookatRotation (.tracestart _outhit_2) (.traceend _outhit_2)) "0.400000,0.400000,0.400000") "AdjustIfPossibleButAlwaysSpawn" 0 0))