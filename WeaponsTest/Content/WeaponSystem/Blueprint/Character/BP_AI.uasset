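; BP_AI is an AI pawn in the weapon system that chases the player once it sees a pawn.
; Its PawnSensing component sets a sensing flag on sight and calls FollowPlayer, which runs AI MoveTo toward the first player's character, whichever pawn was seen.
; The flag is never cleared here, and debug strings print on sighting and on move failure.
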(event OnSeePawn(PawnSensing)
  (params (Pawn :type Pawn%20Object%20Reference))
  (Variables|Default|SetisSensing true)
  (CallFunction|FollowPlayer)
  (Development|PrintString "Hello"))

(event Custom|FollowPlayer
  (if (Variables|Default|GetisSensing)
    (AI|AIMoveTo self "0, 0, 0" (Game|GetPlayerCharacter 0) 5.0 true
      (:OnFail
        (Development|PrintString "fail")))))

(event EventBeginPlay)

(event Collision|EventActorBeginOverlap
  (params (OtherActor :type Actor%20Object%20Reference)))

(event EventTick
  (params (DeltaSeconds :type Float%20%28single-precision%29)))

(fn ConstructionScript)